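; Player for the VolleyBallCrabs game that serves and returns the ball on the Take input.
; Take sends the ball a random move option when play is stopped or the hit box is overlapped, then sets play status.
; Overlapping the box stops play and runs a visible timer counter that teleports the ball to the spawn point past MaxTime.
; Status changes toggle the press-button widget, alongside a coin widget created at start.
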(event `SetSpawnPoint`
  (bind _ball (`self.Ball`))
  ;[1 1 1] Устанавливаем мячик для удара
  (`/Engine/EditorBlueprintResources/StandardMacros.IsValid` _ball
    (:`Is Valid`
      (`self.K2_SetActorLocation` _ball (`SceneComponent.K2_GetComponentLocation` (`self.SpawnPoint`)) false true))))

(event `self.ReceiveBeginPlay`
  (add `self.Status` (delegate `DrawUI`))
  (`self.Status` false)
  (`self.SetSpawnPoint`)
  (bind _returnvalue (`|CreateWidget` "/Game/UI/W_CoinInformation.W_CoinInformation_C"))
  (`UserWidget.AddToViewport` _returnvalue 0))

(event `DrawUI` :!signature `self.Status`
  (params (IsPlay :type Boolean))
  (bind _output_get (set `self.IsPlay` IsPlay))
  (if _output_get
    (`/Engine/EditorBlueprintResources/StandardMacros.IsValid` (stale _returnvalue)
      (:`Is Valid`
        (`Widget.RemoveFromParent` (stale _returnvalue))))
    (else
      (bind _returnvalue (`|CreateWidget` "/Game/UI/W_PressButton.W_PressButton_C"))
      (`UserWidget.AddToViewport` _returnvalue 0))))

(event `InputAction|Take`
  (params (Key :type "Key Structure"))
  (:`Pressed`
    (if (or (`self.Hit`) (not (`self.IsPlay`)))
      (`/Game/Blueprints/VolleyBallCrabs/BP_Ball.MoveBall` (`self.Ball`) (`KismetMathLibrary.RandomIntegerInRange` 0 2))
      (`self.Status` true))))

(event `self.Box.OnComponentBeginOverlap`
  (params (OverlappedComponent :type "PrimitiveComponent Object Reference") (OtherActor :type "Actor Object Reference") (OtherComp :type "PrimitiveComponent Object Reference") (OtherBodyIndex :type Integer) (bFromSweep :type Boolean) (SweepResult :type "HitResult Structure (by ref)"))
  (`SceneComponent.SetVisibility` (`self.TextRender`) true false)
  (set `self.Hit` true)
  (bind _returnvalue (`KismetSystemLibrary.K2_SetTimerDelegate` (delegate `AddTime`) 0.2 true))
  (`self.Status` false))

(event `AddTime`
  (bind _result (`/Engine/EditorBlueprintResources/StandardMacros.IncrementFloat` (`self.Time`))
    (:`  `
      (`TextRenderComponent.K2_SetText` (`self.TextRender`) (`KismetTextLibrary.Conv_DoubleToText` _result "HalfToEven"))
      (if (> _result (`self.MaxTime`))
        (`self.SetSpawnPoint`)))))

(event `self.Box.OnComponentEndOverlap`
  (params (OverlappedComponent :type "PrimitiveComponent Object Reference") (OtherActor :type "Actor Object Reference") (OtherComp :type "PrimitiveComponent Object Reference") (OtherBodyIndex :type Integer))
  (`SceneComponent.SetVisibility` (`self.TextRender`) false false)
  (set `self.Hit` false)
  (bind _output_get (set `self.Time` 0.0))
  (`TextRenderComponent.K2_SetText` (`self.TextRender`) (`KismetTextLibrary.Conv_DoubleToText` _output_get "HalfToEven"))
  (`KismetSystemLibrary.K2_ClearAndInvalidateTimerHandle` (stale `self.Box.OnComponentBeginOverlap` _returnvalue)))

(fn `UserConstructionScript`)